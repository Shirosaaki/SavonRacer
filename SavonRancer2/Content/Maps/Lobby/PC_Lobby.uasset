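; Player controller for the lobby, where each player gets a camera view and a car to customize.
; changeCam stores a spawn transform and relays through onServ to ChangeCamClient, which blends the view, spawns the vehicle and opens UI_Lobby bound to it.
; saveSkin appends default car stats with chosen parts and name to PlayersCars, then passes it to GS_Lobby as ready.
; BeginPlay writes a fresh SG_Game to the "players" slot; releasing F hides the cursor.
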(event `onServ`
  (params (cam :type "Actor Object Reference"))
  (`self.ChangeCamClient` cam))

(event `ChangeCamClient`
  (params (cam :type "Actor Object Reference"))
  (`self.SetViewTargetWithBlend` cam)
  (bind _returnvalue (`|SpawnActorFromClass` "/Game/VehicleAdvBP/Blueprints/VehicleBlueprint.VehicleBlueprint_C" (`self.transform`) "Undefined" "OverrideRootScale" null null))
  (bind _returnvalue_2 (`|CreateWidget` "/Game/Maps/Lobby/UI_Lobby.UI_Lobby_C" null _returnvalue _returnvalue))
  (`UserWidget.AddToViewport` _returnvalue_2 0))

(event `self.ReceiveBeginPlay`
  (bind _returnvalue (`GameplayStatics.CreateSaveGameObject` "/Game/GameInstance/SG_Game.SG_Game_C"))
  (bind _output_get (set `self.GS_Game` _returnvalue))
  (`AsyncActionHandleSaveGame.AsyncSaveGameToSlot` _output_get "players"))

(event `changeCam`
  (params (cam :type "Actor Object Reference") (transform :type "Transform Structure"))
  (set `self.transform` transform)
  (`self.onServ` cam))

(event `Key|F`
  (params (Key :type "Key Structure"))
  (:`Released`
    (set `self.bShowMouseCursor` false)))

(event `saveSkin`
  (params (`Player Parts` :type "Array of /Game/ENNUM_PARTS Enum (by ref)") (Name :type "String (by ref)"))
  (bind _playerscars (`self.playersCars`))
  (`KismetArrayLibrary.Array_Add` _playerscars (make `/Game/VehicleAdvBP/Blueprints/ST_Player` 800.0 1200.0 800.0 0.7 0.85 100.0 0.5 600.0 _ 1.5 1.0 `Player Parts` Name))
  (bind _asgs_lobby (cast `/Game/Maps/Lobby/GS_Lobby` (`GameplayStatics.GetGameState`)))
  (`/Game/Maps/Lobby/GS_Lobby.AddReadyPlayer` _asgs_lobby _playerscars))

(fn `OnRep_playersCars`)

(fn `OnRep_Vehicule BP`)

(fn `UserConstructionScript`)