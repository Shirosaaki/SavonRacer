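; Lobby game mode that gives each joining player a vehicle and a camera view.
; PostLogin records the player, then spawns a vehicle at the PlayerStart named after their index, has PC_Lobby switch to that index's camera and updates GS_Lobby's player count.
; The first player's setup is deferred until addcam fills the camera list, then continues through the same spawn path.
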(event `self.ReceiveBeginPlay`)

(event `add cam`
  (params (cam :type "Array of CameraActor Object Reference"))
  (for _array_element cam
    (`KismetArrayLibrary.Array_AddUnique` (`self.Cameras`) _array_element))
  (bind _returnvalue (`|SpawnActorFromClass` "/Game/VehicleAdvBP/Blueprints/VehicleBlueprint.VehicleBlueprint_C" (`self.GetTransform` (`self.K2_FindPlayerStart` (stale `self.K2_PostLogin` NewPlayer) (`KismetStringLibrary.Conv_IntToString` (stale `self.K2_PostLogin` _returnvalue)))) "Undefined" "OverrideRootScale" null null :!label _label))
  (bind _aspc_lobby (cast `/Game/Maps/Lobby/PC_Lobby` (stale `self.K2_PostLogin` NewPlayer)))
  (`/Game/Maps/Lobby/PC_Lobby.changeCam` _aspc_lobby (`|GetArrayItem` (`self.Cameras`) (stale `self.K2_PostLogin` _returnvalue)) _returnvalue)
  (bind _asgs_lobby (cast `/Game/Maps/Lobby/GS_Lobby` (`GameplayStatics.GetGameState`)))
  (`/Game/Maps/Lobby/GS_Lobby.setNbPlayers` _asgs_lobby (`KismetArrayLibrary.Array_Length` (`self.Players`))))

(event `self.K2_PostLogin`
  (params (NewPlayer :type "PlayerController Object Reference"))
  (bind _returnvalue (`KismetArrayLibrary.Array_AddUnique` (`self.Players`) NewPlayer))
  (if (!= _returnvalue 0)
    (goto _label)))

(fn `UserConstructionScript`)