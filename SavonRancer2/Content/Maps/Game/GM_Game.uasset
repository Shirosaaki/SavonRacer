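; Game mode that runs a turn-based vehicle game, giving each player's car a turn from the player start.
; On BeginPlay it loads saved part lists, spawns vehicles off-map with their parts through OnServer/OnClient events, and attempts default vehicles for missing players.
; Tick snaps a spawned camera actor to the active car's camera.
; A car still stationary when a timer expires is moved away for the next, until the game ends.
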(event `addVehicule`
  (params (NewItem :type "Actor Object Reference (by ref)"))
  (`KismetArrayLibrary.Array_Add` (`self.PlayersCarsGame`) NewItem))

(event `self.ReceiveBeginPlay`
  (bind _numplayer (`self.numPlayer`))
  (bind _returnvalue (`KismetArrayLibrary.Array_Length` (`self.PlayersCarsGame`)))
  (`KismetSystemLibrary.Delay` 2.0)
  (bind _returnvalue_2 (`self.GetNumPlayers`))
  (set `self.numPlayer` _returnvalue_2)
  (bind _returnvalue_3 (`GameplayStatics.LoadGameFromSlot` "players"))
  (bind _assg_game (cast `/Game/GameInstance/SG_Game` _returnvalue_3))
  (for (_array_element _array_index) (`/Game/GameInstance/SG_Game.playersCars` _assg_game)
    (`self.onServer` _array_index (`.PlayerParts_34_1131C4BA4F4A801EF28B2FAB3A3E32CF` (break `/Game/VehicleAdvBP/Blueprints/ST_Player` _array_element))))
  (if (!= _returnvalue _numplayer)
    (for _index (range _returnvalue (+ (+ _numplayer 1) 1))
      (`self.addDefaultVehicule` _index))))

(event `onClient`
  (params (PlayerIndex :type Integer) (Array :type "Array of /Game/ENNUM_PARTS Enum"))
  (bind _returnvalue (`|SpawnActorFromClass` "/Game/VehicleAdvBP/Blueprints/VehicleBlueprint.VehicleBlueprint_C" (`KismetMathLibrary.MakeTransform` (-50000.0 -50000.0 -50000.0)) "Undefined" "OverrideRootScale" (`GameplayStatics.GetPlayerController` PlayerIndex) null))
  (for _array_element Array
    (switch `/Game/ENNUM_PARTS` _array_element
      (:`NewEnumerator5`
        _)
      (:`NewEnumerator0`
        (bind _returnvalue_2 (`|SpawnActorFromClass` "/Game/VehicleAdvBP/Blueprints/parts/Back/Back_1.Back_1_C" (`KismetMathLibrary.MakeTransform` (0.0 0.0 0.0)) "Undefined" "OverrideRootScale" null null))
        (`/Game/VehicleAdvBP/Blueprints/VehicleBlueprint.addParts` _returnvalue _returnvalue_2))
      (:`NewEnumerator1`
        (bind _returnvalue_3 (`|SpawnActorFromClass` "/Game/VehicleAdvBP/Blueprints/parts/Bumper/PA1.PA1_C" (`KismetMathLibrary.MakeTransform` (43.0 0.0 50.0)) "Undefined" "OverrideRootScale" null null))
        (`/Game/VehicleAdvBP/Blueprints/VehicleBlueprint.addParts` _returnvalue _returnvalue_3))
      (:`NewEnumerator2`
        (bind _returnvalue_4 (`|SpawnActorFromClass` "/Game/VehicleAdvBP/Blueprints/parts/ROOF/UP1.UP1_C" (`KismetMathLibrary.MakeTransform` (-25.0 0.0 68.0)) "Undefined" "OverrideRootScale" null null))
        (`/Game/VehicleAdvBP/Blueprints/VehicleBlueprint.addParts` _returnvalue _returnvalue_4))
      (:`NewEnumerator3`
        (bind _returnvalue_5 (`|SpawnActorFromClass` "/Game/VehicleAdvBP/Blueprints/parts/Side/Side_1.Side_1_C" (`KismetMathLibrary.MakeTransform` (0.0 0.0 0.0)) "Undefined" "OverrideRootScale" null null))
        (`/Game/VehicleAdvBP/Blueprints/VehicleBlueprint.addParts` _returnvalue _returnvalue_5))
      (:`NewEnumerator4`
        (bind _returnvalue_6 (`|SpawnActorFromClass` "/Game/VehicleAdvBP/Blueprints/parts/Side/Side_2.Side_2_C" (`KismetMathLibrary.MakeTransform` (0.0 0.0 0.0)) "Undefined" "OverrideRootScale" null null))
        (`/Game/VehicleAdvBP/Blueprints/VehicleBlueprint.addParts` _returnvalue _returnvalue_6)))
    (`self.addVehicule` _returnvalue))
  (`self.SetPlayerProperty`))

(event `onServer`
  (params (PlayerIndex :type Integer) (Array :type "Array of /Game/ENNUM_PARTS Enum (by ref)"))
  (`self.onClient` PlayerIndex Array))

(event `addDefaultVehicule`
  (params (PlayerIndex :type Integer))
  (`self.onServer` PlayerIndex (`self.array`)))

(event `SetPlayerProperty`
  (bind _output (`|GetArrayItem` (`self.PlayersCarsGame`) (`self.playerIndex`)))
  (bind _asvehicle_blueprint (cast `/Game/VehicleAdvBP/Blueprints/VehicleBlueprint` _output))
  (bind _output_get (set `self.getTransformSpawn` (`self.GetTransform` (`self.K2_FindPlayerStart` (`GameplayStatics.GetPlayerController` 0) "0"))))
  (`self.K2_SetActorTransform` _output _output_get false true)
  (set `self.ActualCar` _asvehicle_blueprint)
  (bind _returnvalue (`|SpawnActorFromClass` "/Script/Engine.CameraActor" (`KismetMathLibrary.MakeTransform` (0.0 0.0 0.0)) "Undefined" "OverrideRootScale" null null))
  (set `self.ActualCam` _returnvalue)
  (set `self.initialize` true))

(event `tick-tack`
  (bind _actualcam (`self.ActualCam`))
  (if (`self.initialize`)
    (`self.setCameraSpawn` (`SceneComponent.K2_GetComponentToWorld` (`/Game/VehicleAdvBP/Blueprints/VehicleBlueprint.Camera` (`self.ActualCar`))) _actualcam)
    (bind _aspc_game (cast `/Game/Maps/Game/PC_Game` (`GameplayStatics.GetPlayerController` 0)))
    (`PlayerController.SetViewTargetWithBlend` _aspc_game _actualcam 0.0 "VTBlend_Linear" 0.0 false)
    (if (== (`self.GetVelocity` (`self.ActualCar`)) (0.0 0.0 0.0))
      (if (not (`self.startTimer`))
        (`KismetSystemLibrary.K2_SetTimer` null "EndTimer" 2.0)
        (set `self.startTimer` true)))))

(event `self.ReceiveTick`
  (params (DeltaSeconds :type "Float (single-precision)"))
  (`self.tick-tack`))

(event `setCameraSpawn`
  (params (NewTransform :type "Transform Structure (by ref)") (Target :type "Actor Object Reference"))
  (`self.K2_SetActorTransform` Target NewTransform false true))

(event `EndTimer`
  (if (== (`self.GetVelocity` (`self.ActualCar`)) (0.0 0.0 0.0))
    (`self.ChangePlayer`)))

(event `newCar`
  (params (`Dimension 1` :type Integer) (NewTransform :type "Transform Structure (by ref)"))
  (bind _asvehicle_blueprint (cast `/Game/VehicleAdvBP/Blueprints/VehicleBlueprint` (`|GetArrayItem` (`self.PlayersCarsGame`) `Dimension 1`)))
  (bind _output_get (set `self.ActualCar` _asvehicle_blueprint))
  (`self.setNewVehiculeLocation` _output_get NewTransform))

(event `ChangePlayer`
  (bind _result (`/Engine/EditorBlueprintResources/StandardMacros.IncrementInt` (`self.playerIndex`))
    (:`  `
      (if (< _result (`KismetArrayLibrary.Array_Length` (`self.PlayersCarsGame`)))
        (`self.NewLocationLastVehicule` (`WheeledVehicle.Mesh` (`self.ActualCar`)))
        (`self.newCar` _result (`self.getTransformSpawn`))
        (else
          (`self.EndGame`))))))

(event `setNewVehiculeLocation`
  (params (Target :type "Actor Object Reference") (NewTransform :type "Transform Structure (by ref)"))
  (`SceneComponent.K2_SetWorldTransform` (`Actor.RootComponent` Target) NewTransform false true))

(event `NewLocationLastVehicule`
  (params (Target :type "SceneComponent Object Reference"))
  (`SceneComponent.K2_SetWorldLocation` Target (-5000.0 -5000.0 -5000.0) false true))

(event `EndGame`
  (`KismetSystemLibrary.PrintString` "End" true true (struct :`G` 0.66 :`B` 1.0 :`A` 1.0) 50.0))

(fn `UserConstructionScript`)